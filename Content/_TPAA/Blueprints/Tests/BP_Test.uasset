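; BP_Test is a scratch test actor holding samples of Blueprint node types, variable types, containers, functions, a macro, collapsed graphs and an event dispatcher.
; At runtime it prints its display name on BeginPlay and fires its event dispatcher when an actor overlaps it.
; Most other nodes, including the dispatcher binding, variable setters and flow-control samples, are disconnected and never run.
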(event Custom|NewEventDispatcher_Event
  (params (NewParam :type Boolean)))

(event EventBeginPlay
  (Development|PrintString (Utilities|GetDisplayName self) true false "(R=1.000000,G=0.000000,B=0.556704,A=1.000000)" 5.0))

(event Collision|EventActorBeginOverlap
  (params (OtherActor :type Actor%20Object%20Reference))
  (Default|CallNewEventDispatcher true))

(event EventTick
  (params (DeltaSeconds :type Float%20%28single-precision%29)))

(fn ConstructionScript)

(fn NewFunction)

(fn NewFunction0)

(fn NewFunction1
  (Development|PrintString "Hello"))

(event Custom|CustomEvent
  (params (NewParam :type Boolean))
  (CallFunction|NewFunction1)
  (CallFunction|NewFunction0))