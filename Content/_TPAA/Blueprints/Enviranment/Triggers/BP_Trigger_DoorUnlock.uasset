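; Trigger actor that unlocks the locked doors linked to it when an actor begins overlapping it.
; After running the parent overlap logic, it checks that LinkedLockedDoors has a first entry, then calls UnlockDoor on every linked door.
; A DoOnce makes the unlock fire only once, and this Blueprint applies no filter on the overlapping actor.
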(event EventBeginPlay
  (|CallParentFunction) ; This node is disabled and will not be called.\nDrag off pins to build functionality.
)

(event Collision|EventActorBeginOverlap
  (params (OtherActor :type Actor%20Object%20Reference))
  (|CallParentFunction OtherActor)
  (if (Utilities|Array|IsValidIndex (Variables|Default|GetLinkedLockedDoors))
    (Utilities|FlowControl|DoOnce false
      (:Completed
        (for _array_element (Variables|Default|GetLinkedLockedDoors)
          (Default|UnlockDoor _array_element))))))

(event EventTick
  (params (DeltaSeconds :type Float%20%28single-precision%29))
  (|CallParentFunction DeltaSeconds) ; This node is disabled and will not be called.\nDrag off pins to build functionality.
)

(fn ConstructionScript
  (|CallParentFunction))