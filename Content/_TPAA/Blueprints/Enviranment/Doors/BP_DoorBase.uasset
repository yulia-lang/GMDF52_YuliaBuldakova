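; Base interactable hinged door that toggles open and closed, swinging in a direction set by which side the interacting actor is on.
; Interact takes the sign of a dot product against the Arrow, then a timeline drives the pivot's yaw, reversing along the stored sign to close.
; Door mesh collision and repeat triggers are blocked during motion.
; The construction script applies the initial open state and box collision size.
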(event Custom|OpenDoor
  (if (not (Variables|Default|GetbInProgress))
    (if (not (Variables|Default|GetIsDoorOpen))
      (CallFunction|UpdateinProgress true)
      (bind (_direction _dooropenprogress) (Timeline|DoorProgressTimeline PlayFromStart)
        (:Update
          (Transformation|SetRelativeRotation (Variables|Default|GetDoorScene) (Math|Rotator|MakeRotator 0.0 0.0 (* (Variables|Default|GetMaxDoorOpenAngle) _dooropenprogress (Math|Float|SelectFloat (Variables|Default|GetPreviousDotProduct) (Variables|Default|GetCurrentDotProduct) (Variables|Default|GetIsDoorOpen)))) false false))
        (:Finished
          (Variables|Default|SetPreviousDotProduct (Variables|Default|GetCurrentDotProduct))
          (CallFunction|UpdateinProgress false)
          (switch Utilities|FlowControl|Switch|SwitchonETimelineDirection _direction
            (:Forward
              (Variables|Default|SetIsDoorOpen true))
            (:Backward
              (Variables|Default|SetIsDoorOpen false))))))))

(event Custom|CloseDoor
  (if (not (Variables|Default|GetbInProgress))
    (if (Variables|Default|GetIsDoorOpen)
      (CallFunction|UpdateinProgress true)
      (bind (_direction _dooropenprogress) (Timeline|DoorProgressTimeline ReverseFromEnd)
        (:Update
          (Transformation|SetRelativeRotation (Variables|Default|GetDoorScene) (Math|Rotator|MakeRotator 0.0 0.0 (* (Variables|Default|GetMaxDoorOpenAngle) _dooropenprogress (Math|Float|SelectFloat (Variables|Default|GetPreviousDotProduct) (Variables|Default|GetCurrentDotProduct) (Variables|Default|GetIsDoorOpen)))) false false))
        (:Finished
          (Variables|Default|SetPreviousDotProduct (Variables|Default|GetCurrentDotProduct))
          (CallFunction|UpdateinProgress false)
          (switch Utilities|FlowControl|Switch|SwitchonETimelineDirection _direction
            (:Forward
              (Variables|Default|SetIsDoorOpen true))
            (:Backward
              (Variables|Default|SetIsDoorOpen false))))))))

(event EventBeginPlay
  (Components|Timeline|SetPlayRate (Variables|Default|GetDoorProgressTimeline) (Variables|Default|GetDoorOpenSpeed)))

(fn ConstructionScript
  (Utilities|FlowControl|Sequence
    (:then_0
      (CallFunction|ConfigureOpenDooronConstruct))
    (:then_1
      (CallFunction|UpdateBoxExtent))))

(fn UpdateDoorVisual
  (if (Variables|Default|GetIsDoorOpen)
    (CallFunction|CloseDoor)
    (else
      (CallFunction|OpenDoor))))

(fn SwitchDoorOpen
  (Variables|Default|SetIsDoorOpen (not (Variables|Default|GetIsDoorOpen)))
  (CallFunction|UpdateDoorVisual))

(fn UpdateinProgress
  (params (bInProgress :type Boolean))
  (Variables|Default|SetbInProgress bInProgress)
  (Collision|SetCollisionEnabled (Variables|Default|GetDoorMash) (select (Variables|Default|GetbInProgress) "NoCollision" "QueryAndPhysics")))

(fn DoorDotProduct
  (bind _bdebugenable (Variables|Debug|GetbDebugEnable))
  (bind _arrow (Variables|Default|GetArrow))
  (bind _actorofinteraction (Variables|Default|GetActorOfInteraction))
  (bind _rootcomponent (Variables|/Script/Engine.Actor|GetRootComponent _actorofinteraction))
  (bind _outdotproductresult (CallFunction|DotProductOfTwoComponents _arrow _rootcomponent _bdebugenable))
  (bind _returnvalue (> _outdotproductresult 0.0))
  (bind _returnvalue_2 (Math|Float|SelectFloat 1.0 -1.0 _returnvalue))
  (CallFunction|PringStringCustom (Utilities|String|Append (Utilities|String|ToString(Float) _outdotproductresult) "///  " (Utilities|String|ToString(Float) _returnvalue_2)) (Variables|Debug|GetbDebugEnable) "(R=0.000000,G=1.000000,B=0.020157,A=1.000000)" 3.0 "None")
  (return _returnvalue_2))

(fn UpdateBoxExtent
  ;[0.15 0.15 0.15 0.5] Locations update on constuction
  (Components|Box|SetBoxExtent (Variables|Default|GetDoorBoxColLision) (Variables|Default|GetDoorBoxCollisionExtent) true)
  (Transformation|SetRelativeLocation (Variables|Default|GetDoorBoxColLision) (Math|Vector|MakeVector 0.0 0.0 (.z (Variables|Default|GetDoorBoxCollisionExtent))) false false))

(fn ConfigureOpenDooronConstruct
  (Transformation|SetRelativeRotation (Variables|Default|GetDoorScene) (Math|Rotator|MakeRotator 0.0 0.0 (Math|Float|SelectFloat (Variables|Default|GetMaxDoorOpenAngle) 0.0 (Variables|Default|GetIsDoorOpen))) false false))

(fn Interact
  (params (InteractActor :type Actor%20Object%20Reference))
  (Variables|Default|SetActorOfInteraction InteractActor)
  (Variables|Default|SetCurrentDotProduct (CallFunction|DoorDotProduct))
  (CallFunction|UpdateDoorVisual)
  (return true))