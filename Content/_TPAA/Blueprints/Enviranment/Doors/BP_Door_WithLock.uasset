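; BP_Door_WithLock is a lockable child of a door Blueprint that cannot open visually while locked.
; While locked, it forces a closed start on construction, shows front and back lock icons, and replaces the parent's visual update with a timeline-driven yaw jiggle scaled by CurrentDotProduct.
; UnlockDoor clears the lock and swaps both icons to open-lock meshes, then sets them visible after a short delay.
; Its Interact override always returns false.
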(event Custom|TryOpenLockDoor
  (bind _doorlockedtryingprogress (Timeline|LockedFeedbackTimeline PlayFromStart)
    (:Update
      (Transformation|SetRelativeRotation (Variables|Default|GetDoorScene) (Math|Rotator|MakeRotator 0.0 0.0 (* (Variables|Default|GetLockedDoorAngle) _doorlockedtryingprogress (Variables|Default|GetCurrentDotProduct))) false false))))

(event Custom|UnlockFeedback
  (Components|StaticMesh|SetStaticMesh (Variables|Default|GetIcon_LockClosedMeshF) "/Game/Polygon_Prototype/Meshes/Icons/SM_Icon_Lock_Open_01.SM_Icon_Lock_Open_01")
  (Components|StaticMesh|SetStaticMesh (Variables|Default|GetIcon_LockClosedMeshB) "/Game/Polygon_Prototype/Meshes/Icons/SM_Icon_Lock_Open_01.SM_Icon_Lock_Open_01")
  (Utilities|FlowControl|Delay 2.0)
  (Rendering|SetVisibility (Variables|Default|GetIcon_LockClosedMeshF) true false))

(fn ConstructionScript
  (|CallParentFunction)
  (Rendering|SetVisibility (Variables|Default|GetIcon_LockClosedMeshF) (Variables|Default|GetbIsDoorLocked) false))

(fn UpdateDoorVisual
  (if (not (Variables|Default|GetbIsDoorLocked))
    (|CallParentFunction)
    (else
      (CallFunction|TryOpenLockDoor))))

(fn ConfigureOpenDooronConstruct
  (if (Variables|Default|GetbIsDoorLocked)
    (Variables|Default|SetIsDoorOpen (not (Variables|Default|GetbIsDoorLocked))))
  (|CallParentFunction))

(fn Interact
  (params (InteractActor :type Actor%20Object%20Reference))
  (return false))

(fn UnlockDoor
  (Variables|Default|SetbIsDoorLocked false)
  (CallFunction|UnlockFeedback))