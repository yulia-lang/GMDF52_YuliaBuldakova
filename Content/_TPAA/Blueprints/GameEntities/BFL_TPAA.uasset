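; BFL_TPAA is a Blueprint function library of debug and vector helpers for TPAA game entities.
; DotProductOfTwoComponents returns the dot product of one component's forward vector and the normalized direction to another, measuring how directly it faces that component.
; An optional debug flag draws arrows for both vectors.
; PringStringCustom wraps PrintString with log output disabled, and TestLibraryFunction is an empty stub.
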(fn PringStringCustom
  (params (InString :type String) (bPrintToScreen :type Boolean) (TextColor :type Linear%20Color%20Structure) (Duration :type Float%20%28double-precision%29) (Key :type Name))
  (Development|PrintString 0 InString bPrintToScreen false TextColor Duration Key))

(fn TestLibraryFunction
  (return))

(fn DotProductOfTwoComponents
  (params (InSceneComponentFromDotProduct :type Scene%20Component%20Object%20Reference) (InSceneComponentToDotProduct :type Scene%20Component%20Object%20Reference) (bInDebugEnable :type Boolean))
  (bind _returnvalue (Transformation|GetWorldLocation InSceneComponentFromDotProduct))
  (Utilities|FlowControl|Sequence
    (:then_0
      (if bInDebugEnable
        (Rendering|Debug|DrawDebugArrow 0 (Transformation|GetWorldLocation InSceneComponentFromDotProduct) (Transformation|GetWorldLocation InSceneComponentToDotProduct) 15.0 "(R=0.000000,G=0.139287,B=1.000000,A=1.000000)" 3.0 4.0)
        (Rendering|Debug|DrawDebugArrow 0 _returnvalue (+ _returnvalue (* (Math|Vector|GetForwardVector InSceneComponentFromDotProduct) 1e+02)) 15.0 "(R=1.000000,G=0.000867,B=0.219687,A=1.000000)" 3.0 4.0)))
    (:then_1
      (return (Math|Vector|DotProduct (Math|Vector|Normalize (- (Transformation|GetWorldLocation InSceneComponentToDotProduct) (Transformation|GetWorldLocation InSceneComponentFromDotProduct))) (Math|Vector|GetForwardVector InSceneComponentFromDotProduct))))))